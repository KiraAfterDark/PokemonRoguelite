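; GAME_Pokemon_BP represents a single Pokemon in the game, initialised from a data entry.
; Init stores the data, copies its base stats, name and attacks, and constructs a GAME_Health_BP object seeded with the base HP.
; Health is delegated to that separate object rather than tracked on the Pokemon itself.
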(fn `Init`
  (params (Data :type "/Game/Blueprints/Data/Pokemon/PKM_Pokemon_DATA Object Reference"))
  (bind _stats_hp (break `/Game/Blueprints/Data/Pokemon/PKM_StatBlock_STRT` (`self.Stats`)))
  (bind _data (`self.Data`))
  (bind _output_get (set `self.Data` Data))
  (set `self.Stats` (`/Game/Blueprints/Data/Pokemon/PKM_Pokemon_DATA.Base Stats` _output_get))
  (bind _returnvalue (`|GenericCreateObject` "/Game/Blueprints/Gameplay/GAME_Health_BP.GAME_Health_BP_C"))
  (bind _output_get_2 (set `self.Health` _returnvalue))
  (`/Game/Blueprints/Gameplay/GAME_Health_BP.Init` _output_get_2 _stats_hp)
  (set `self.Name` (`/Game/Blueprints/Data/Pokemon/PKM_Pokemon_DATA.Name` _data))
  (set `self.Attacks` (`/Game/Blueprints/Data/Pokemon/PKM_Pokemon_DATA.Attack` _data)))