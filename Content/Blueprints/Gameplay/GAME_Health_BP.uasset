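; GAME_Health_BP is a health Blueprint that tracks current and maximum health for whatever uses it.
; Init sets both values from a supplied HP stat.
; Damage and Heal clamp current health between zero and the maximum, then fire the OnHealthChange dispatcher.
; A getter returns current health as a fraction of the maximum.
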(fn `Damage`
  (params (Damage :type Integer))
  (set `self.Current Health` (`KismetMathLibrary.Max` (- (`self.Current Health`) Damage)))
  (`self.On Health Change`))

(fn `Get Normalized Health`
  (returns (`Normalized Health` :type "Float (double-precision)"))
  (return (/ (`KismetMathLibrary.Conv_IntToDouble` (`self.Current Health`)) (`KismetMathLibrary.Conv_IntToDouble` (`self.Max Health`)))))

(fn `Heal`
  (params (Heal :type Integer))
  (set `self.Current Health` (`KismetMathLibrary.Min` (+ Heal (`self.Current Health`)) (`self.Max Health`)))
  (`self.On Health Change`))

(fn `Init`
  (params (`Hp Stat` :type Integer))
  (bind _output_get (set `self.Max Health` `Hp Stat`))
  (set `self.Current Health` _output_get))