(fn `Create Action`
  (params (Source :type "/Game/Blueprints/Battle/Pokemon/BTL_Pokemon_BP Object Reference") (Target :type "/Game/Blueprints/Battle/Pokemon/BTL_Pokemon_BP Object Reference") (Attack :type "/Game/Blueprints/Data/Attacks/ATK_Attack_DATA Object Reference"))
  (set `self.Source` Source)
  (set `self.Target` Target)
  (set `self.Attack` Attack))

(fn `Finish Action`
  (`self.On Action Completed`))

(fn `Get Priority`
  (returns (Priority :type "Float (double-precision)"))
  (bind _priority (`parent.Get Priority`))
  (return _priority))

(fn `Perform Action`
  (`KismetSystemLibrary.LogString` "Attack Performing")
  (`KismetSystemLibrary.K2_SetTimerDelegate` (`|CreateDelegate` :!event `Finish Action`) 1.0)
  (bind _target (`self.Target`)
    (:`then`
      (`/Game/Blueprints/Battle/Pokemon/BTL_Pokemon_BP.Damage` _target (`/Game/Blueprints/Data/Attacks/ATK_Attack_DATA.Power` (`self.Attack`))))
    (:`else`)))